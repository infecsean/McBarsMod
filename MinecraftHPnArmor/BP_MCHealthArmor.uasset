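; Mod actor that shows a Minecraft-style health and armor bar HUD for the local player, with a mod hub settings page.
; On BeginPlay it retries until the player is valid, creates both widgets, then applies saved scale and position.
; HealthComponent events drive bar updates, brief hit flashes and low or regenerating animation states.
; Settings changes move or scale the bars live and save when the hub closes.
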(event Custom|OnArmorChange
  (params (Health :type Float%20%28single-precision%29))
  (bind _player_char_ref (Variables|Default|GetPlayer%20Char%20Ref))
  (bind _player_char_ref_2 (Variables|Default|GetPlayer%20Char%20Ref))
  (bind _hud_ref (Variables|Default|GetHUD%20Ref))
  (bind _hud_ref_2 (Variables|Default|GetHUD%20Ref))
  (bind _healthcomponent (Variables|/Script/FSD.PlayerCharacter|GetHealthComponent _player_char_ref))
  (bind _healthcomponent_2 (Variables|/Script/FSD.PlayerCharacter|GetHealthComponent _player_char_ref_2))
  (bind _returnvalue (Class|HealthComponent|GetArmorPct _healthcomponent))
  (bind _returnvalue_2 (Class|HealthComponent|GetArmorPct _healthcomponent_2))
  (if (and (> _returnvalue_2 (Variables|Default|GetoldArmor)) (< _returnvalue_2 0.95))
    (Variables|/Game/MinecraftHPnArmor/WBP_MCHealthArmor.WBP_MCHealthArmor_C|SetAnimStateArmor _hud_ref_2 "NewEnumerator2")
    (elif (< _returnvalue_2 0.2)
      (Variables|/Game/MinecraftHPnArmor/WBP_MCHealthArmor.WBP_MCHealthArmor_C|SetAnimStateArmor _hud_ref "NewEnumerator1")
      (else
        (Variables|/Game/MinecraftHPnArmor/WBP_MCHealthArmor.WBP_MCHealthArmor_C|SetAnimStateArmor _hud_ref "NewEnumerator0"))))
  (Default|UpdateArmor _hud_ref_2 _returnvalue false)
  (Variables|Default|SetoldArmor _returnvalue))

(event Custom|OnPlayerDamageTaken
  (params (amount :type Float%20%28single-precision%29))
  (bind _player_char_ref (Variables|Default|GetPlayer%20Char%20Ref))
  (bind _healthcomponent (Variables|/Script/FSD.PlayerCharacter|GetHealthComponent _player_char_ref))
  (bind _returnvalue (Class|HealthComponentBase|GetHealthPct _healthcomponent))
  (Default|UpdateHealth (Variables|Default|GetHUD%20Ref) _returnvalue true)
  (Utilities|FlowControl|Delay 0.1)
  (Default|UpdateHealth (Variables|Default|GetHUD%20Ref) _returnvalue false))

(event Custom|OnHUDToggle
  (params (InHudVisible :type Boolean))
  (bind _hud_ref (Variables|Default|GetHUD%20Ref))
  (if InHudVisible
    (Widget|SetVisibility _hud_ref "Visible")
    (else
      (Widget|SetVisibility _hud_ref "Collapsed"))))

(event Custom|OnHealthRegen
  (params (isRegenerating :type Boolean))
  (bind _hud_ref (Variables|Default|GetHUD%20Ref))
  (if isRegenerating
    (Variables|/Game/MinecraftHPnArmor/WBP_MCHealthArmor.WBP_MCHealthArmor_C|SetAnimStateHealth (Variables|Default|GetHUD%20Ref) "NewEnumerator2")
    (elif (< (Class|HealthComponentBase|GetHealthPct (Variables|/Script/FSD.PlayerCharacter|GetHealthComponent (Variables|Default|GetPlayer%20Char%20Ref))) 0.2)
      (Variables|/Game/MinecraftHPnArmor/WBP_MCHealthArmor.WBP_MCHealthArmor_C|SetAnimStateHealth _hud_ref "NewEnumerator1")
      (else
        (Variables|/Game/MinecraftHPnArmor/WBP_MCHealthArmor.WBP_MCHealthArmor_C|SetAnimStateHealth _hud_ref "NewEnumerator0")))))

(event Custom|OnArmorDamage
  (params (amount :type Float%20%28single-precision%29))
  (bind _player_char_ref (Variables|Default|GetPlayer%20Char%20Ref))
  (bind _healthcomponent (Variables|/Script/FSD.PlayerCharacter|GetHealthComponent _player_char_ref))
  (bind _returnvalue (Class|HealthComponent|GetArmorPct _healthcomponent))
  (Default|UpdateArmor (Variables|Default|GetHUD%20Ref) _returnvalue true)
  (Utilities|FlowControl|Delay 0.2)
  (Default|UpdateArmor (Variables|Default|GetHUD%20Ref) _returnvalue false))

(event Custom|OnPlayerHealthChanged
  (params (Health :type Float%20%28single-precision%29))
  (bind _hud_ref (Variables|Default|GetHUD%20Ref))
  (bind _player_char_ref (Variables|Default|GetPlayer%20Char%20Ref))
  (bind _healthcomponent (Variables|/Script/FSD.PlayerCharacter|GetHealthComponent _player_char_ref))
  (bind _returnvalue (Class|HealthComponentBase|GetHealthPct _healthcomponent))
  (Default|UpdateHealth (Variables|Default|GetHUD%20Ref) _returnvalue false)
  (if (< _returnvalue 0.2)
    (Variables|/Game/MinecraftHPnArmor/WBP_MCHealthArmor.WBP_MCHealthArmor_C|SetAnimStateHealth (Variables|Default|GetHUD%20Ref) "NewEnumerator1")
    (elif (Class|PlayerHealthComponent|GetIsHealthRegenerating (Variables|/Script/FSD.PlayerCharacter|GetHealthComponent (Variables|Default|GetPlayer%20Char%20Ref)))
      (Variables|/Game/MinecraftHPnArmor/WBP_MCHealthArmor.WBP_MCHealthArmor_C|SetAnimStateHealth _hud_ref "NewEnumerator2")
      (else
        (Variables|/Game/MinecraftHPnArmor/WBP_MCHealthArmor.WBP_MCHealthArmor_C|SetAnimStateHealth _hud_ref "NewEnumerator0")))))

(event Custom|OnWidgetScaleValChanged
  (params (InValue :type Float%20%28single-precision%29))
  (Widget|Transform|SetRenderScale (Variables|/Game/MinecraftHPnArmor/WBP_MCHealthArmor.WBP_MCHealthArmor_C|GetBarContainer (Variables|Default|GetHUD%20Ref)) (Math|Vector2D|MakeVector2D InValue InValue)))

(event Custom|OnWidgetPosXChange
  (params (InValue :type Float%20%28single-precision%29))
  (bind _hud_ref (Variables|Default|GetHUD%20Ref))
  (bind _barcontainer (Variables|/Game/MinecraftHPnArmor/WBP_MCHealthArmor.WBP_MCHealthArmor_C|GetBarContainer _hud_ref))
  (bind _returnvalue (Class|WidgetLayoutLibrary|SlotasCanvasSlot _barcontainer))
  (Class|CanvasPanelSlot|SetPosition _returnvalue (Math|Vector2D|MakeVector2D InValue (.Y (Math|Vector2D|BreakVector2D (Class|CanvasPanelSlot|GetPosition _returnvalue))))))

(event Custom|OnWidgetPosYChange
  (params (InValue :type Float%20%28single-precision%29))
  (bind _hud_ref (Variables|Default|GetHUD%20Ref))
  (bind _barcontainer (Variables|/Game/MinecraftHPnArmor/WBP_MCHealthArmor.WBP_MCHealthArmor_C|GetBarContainer _hud_ref))
  (bind _returnvalue (Class|WidgetLayoutLibrary|SlotasCanvasSlot _barcontainer))
  (Class|CanvasPanelSlot|SetPosition _returnvalue (Math|Vector2D|MakeVector2D (.X (Math|Vector2D|BreakVector2D (Class|CanvasPanelSlot|GetPosition _returnvalue))) InValue)))

(event EventBeginPlay
  (bind _returnvalue (Class|GameFunctionLibrary|GetLocalPlayerCharacter))
  (Utilities|IsValid _returnvalue :!label _label
    (:Is%20Valid
      (Variables|Default|SetPlayer%20Char%20Ref _returnvalue)
      (Utilities|CreateHUD
        (:out
          (CallFunction|LoadSave)
          (CallFunction|LoadSaveSettings)
          (Utilities|FlowControl|Sequence
            (:then_0
              (EventDispatchers|AssignOnValueChanged (Variables|/Game/MinecraftHPnArmor/WBP_McBars_Settings.WBP_McBars_Settings_C|GetWidgetScale (Variables|Default|GetHub%20Page)) (delegate Custom|OnWidgetScaleValChanged))
              (EventDispatchers|AssignOnValueChanged (Variables|/Game/MinecraftHPnArmor/WBP_McBars_Settings.WBP_McBars_Settings_C|GetWidgetPosX (Variables|Default|GetHub%20Page)) (delegate Custom|OnWidgetPosXChange))
              (EventDispatchers|AssignOnValueChanged (Variables|/Game/MinecraftHPnArmor/WBP_McBars_Settings.WBP_McBars_Settings_C|GetWidgetPosY (Variables|Default|GetHub%20Page)) (delegate Custom|OnWidgetPosYChange))
              (EventDispatchers|AssignOnHUDVisibilityChanged (Class|FSDHUD|GetFSDHUD (CallFunction|GetLocalPlayerController)) (delegate Custom|OnHUDToggle)))
            (:then_1
              (EventDispatchers|AssignOnDamageTaken (Variables|/Script/FSD.PlayerCharacter|GetHealthComponent (Variables|Default|GetPlayer%20Char%20Ref)) (delegate Custom|OnPlayerDamageTaken))
              (EventDispatchers|AssignOnHealthRegeneratingChanged (Variables|/Script/FSD.PlayerCharacter|GetHealthComponent (Variables|Default|GetPlayer%20Char%20Ref)) (delegate Custom|OnHealthRegen))
              (EventDispatchers|AssignOnHealthChanged (Variables|/Script/FSD.PlayerCharacter|GetHealthComponent (Variables|Default|GetPlayer%20Char%20Ref)) (delegate Custom|OnPlayerHealthChanged)))
            (:then_2
              (EventDispatchers|AssignOnArmorDamaged (Variables|/Script/FSD.PlayerCharacter|GetHealthComponent (Variables|Default|GetPlayer%20Char%20Ref)) (delegate Custom|OnArmorDamage))
              (EventDispatchers|AssignOnArmorChanged (Variables|/Script/FSD.PlayerCharacter|GetHealthComponent (Variables|Default|GetPlayer%20Char%20Ref)) (delegate Custom|OnArmorChange)))))))
    (:Is%20Not%20Valid
      (Utilities|FlowControl|Delay 0.2)
      (goto _label))))

(event Collision|EventActorBeginOverlap
  (params (OtherActor :type Actor%20Object%20Reference)))

(event EventTick
  (params (DeltaSeconds :type Float%20%28single-precision%29)))

(event EventModHubClosed
  (CallFunction|SaveSettings))

(event EventModHubOpened
  (bind _hub_page (Variables|Default|GetHub%20Page))
  (bind _mcbars_settings (Variables|Default|GetMcBars%20Settings))
  (bind _hub_page_2 (Variables|Default|GetHub%20Page))
  (bind _barposition (Variables|/Game/MinecraftHPnArmor/SAV_McBarSettings.SAV_McBarSettings_C|GetBarPosition _mcbars_settings))
  (bind _widgetscale (Variables|/Game/MinecraftHPnArmor/WBP_McBars_Settings.WBP_McBars_Settings_C|GetWidgetScale _hub_page))
  (bind _widgetposx (Variables|/Game/MinecraftHPnArmor/WBP_McBars_Settings.WBP_McBars_Settings_C|GetWidgetPosX _hub_page_2))
  (bind _widgetposy (Variables|/Game/MinecraftHPnArmor/WBP_McBars_Settings.WBP_McBars_Settings_C|GetWidgetPosY _hub_page_2))
  (bind (_x _y) (Math|Vector2D|BreakVector2D _barposition))
  (Variables|/Game/DRGLib/UITemplates/Spinbox/LIB_WT_Spinbox.LIB_WT_Spinbox_C|SetValue _widgetscale (Variables|/Game/MinecraftHPnArmor/SAV_McBarSettings.SAV_McBarSettings_C|GetBarScale (Variables|Default|GetMcBars%20Settings)))
  (Default|UpdateDisplayedValues _widgetscale)
  (Variables|/Game/DRGLib/UITemplates/Spinbox/LIB_WT_Spinbox.LIB_WT_Spinbox_C|SetValue _widgetposx _x)
  (Default|UpdateDisplayedValues _widgetposx)
  (Variables|/Game/DRGLib/UITemplates/Spinbox/LIB_WT_Spinbox.LIB_WT_Spinbox_C|SetValue _widgetposy _y)
  (Default|UpdateDisplayedValues _widgetposy))

(fn ConstructionScript)

(fn LoadSave
  (bind _returnvalue (SaveGame|DoesSaveGameExist (Variables|Default|GetSave%20File%20Name)))
  (if _returnvalue
    (bind _returnvalue_2 (SaveGame|LoadGamefromSlot (Variables|Default|GetSave%20File%20Name)))
    (bind _assav_mc_bar_settings (Utilities|Casting|CastToSAV_McBarSettings _returnvalue_2))
    (Variables|Default|SetMcBars%20Settings _assav_mc_bar_settings)
    (else
      (bind _returnvalue_3 (SaveGame|CreateSaveGameObject "/Game/MinecraftHPnArmor/SAV_McBarSettings.SAV_McBarSettings_C"))
      (Variables|Default|SetMcBars%20Settings _returnvalue_3))))

(fn SaveSettings
  (bind _mcbars_settings (Variables|Default|GetMcBars%20Settings))
  (Variables|/Game/MinecraftHPnArmor/SAV_McBarSettings.SAV_McBarSettings_C|SetBarScale _mcbars_settings (.X (Math|Vector2D|BreakVector2D (.Scale (Utilities|Struct|BreakWidgetTransform (Variables|/Script/UMG.Widget|GetRenderTransform (Variables|/Game/MinecraftHPnArmor/WBP_MCHealthArmor.WBP_MCHealthArmor_C|GetBarContainer (Variables|Default|GetHUD%20Ref))))))))
  (Variables|/Game/MinecraftHPnArmor/SAV_McBarSettings.SAV_McBarSettings_C|SetBarPosition _mcbars_settings (Class|CanvasPanelSlot|GetPosition (Class|WidgetLayoutLibrary|SlotasCanvasSlot (Variables|/Game/MinecraftHPnArmor/WBP_MCHealthArmor.WBP_MCHealthArmor_C|GetBarContainer (Variables|Default|GetHUD%20Ref)))))
  (SaveGame|SaveGametoSlot (Variables|Default|GetMcBars%20Settings) (Variables|Default|GetSave%20File%20Name)))

(fn LoadSaveSettings
  (bind _mcbars_settings (Variables|Default|GetMcBars%20Settings))
  (bind _hud_ref (Variables|Default|GetHUD%20Ref))
  (bind _barscale (Variables|/Game/MinecraftHPnArmor/SAV_McBarSettings.SAV_McBarSettings_C|GetBarScale _mcbars_settings))
  (bind _barcontainer (Variables|/Game/MinecraftHPnArmor/WBP_MCHealthArmor.WBP_MCHealthArmor_C|GetBarContainer _hud_ref))
  (Widget|Transform|SetRenderScale _barcontainer (Math|Vector2D|MakeVector2D _barscale _barscale))
  (Class|CanvasPanelSlot|SetPosition (Class|WidgetLayoutLibrary|SlotasCanvasSlot _barcontainer) (Variables|/Game/MinecraftHPnArmor/SAV_McBarSettings.SAV_McBarSettings_C|GetBarPosition _mcbars_settings)))

(fn GetModInfo
  (return "Minecraft Hp/Armor" "stag" "1.0"))

(fn GetModPages
  (return (Utilities|Array|MakeArray (Variables|Default|GetHub%20Page))))